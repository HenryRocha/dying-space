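; BP_NPC is an NPC Blueprint that tracks health and death state.
; On BeginPlay it sets current health to max health.
; Taking damage flags the player as found, subtracts from health and, at zero or below, marks the NPC dead and prints a debug message.
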(event `self.ReceiveBeginPlay`
  (set `self.CurrentHealth` (`self.MaxHealth`)))

(event `/Game/AI/Blueprints/BP_DamageSystem.TakeDamage`
  (params (BoneName :type Name) (Damage :type "Float (single-precision)"))
  (set `self.PlayerFound` true)
  (bind _output_get (set `self.CurrentHealth` (- (`self.CurrentHealth`) Damage)))
  (if (<= _output_get 0.0)
    (set `self.isDead` true)
    (`KismetSystemLibrary.PrintString` "NPC has died!")))

(fn `UserConstructionScript`)