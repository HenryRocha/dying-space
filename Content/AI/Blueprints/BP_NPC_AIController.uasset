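; AI controller for BP_NPC that sends it to a waypoint and has it chase the player once found.
; On BeginPlay it caches the NPC and its waypoints, then moves to the current waypoint, with no onward patrol step after arrival.
; A looping timer polls the NPC's PlayerFound flag to trigger a chase toward player 0, and clears itself when the NPC is dead.
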(event `self.ReceiveBeginPlay`
  (bind _asbp_npc (cast `/Game/AI/Blueprints/BP_NPC` (`self.K2_GetPawn`)))
  (set `self.AIReference` _asbp_npc)
  (set `self.WaypointsReference` (`/Game/AI/Blueprints/BP_NPC.Waypoints` _asbp_npc))
  (bind _returnvalue (`KismetSystemLibrary.K2_SetTimer` null "CheckPlayer" 0.25 true))
  (set `self.Clear Time` _returnvalue)
  (`|AIMoveTo` null (0.0 0.0 0.0) (`|GetArrayItem` (`self.WaypointsReference`) (`self.CurrentWaypoint`))
    (:`OnSuccess`
      (`KismetSystemLibrary.Delay` 1.25))))

(event `OnChase`
  (`|AIMoveTo` null (0.0 0.0 0.0) (`GameplayStatics.GetPlayerCharacter` 0) 200.0))

(event `CheckPlayer`
  (bind _aireference (`self.AIReference`))
  (if (`/Game/AI/Blueprints/BP_NPC.isDead` _aireference)
    (`KismetSystemLibrary.K2_ClearAndInvalidateTimerHandle` (`self.Clear Time`))
    (else
      (bind _output_get (set `self.PlayerFound` (`/Game/AI/Blueprints/BP_NPC.PlayerFound` _aireference)))
      (if _output_get
        (`self.OnChase`)))))

(fn `UserConstructionScript`)