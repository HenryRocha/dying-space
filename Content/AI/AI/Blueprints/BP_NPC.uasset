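; BP_NPC is an AI character that tracks its health and whether it has detected the player.
; PawnSensing sets PlayerFound when it sees BP_MainCharacter, and a retriggerable delay clears the flag shortly after the last sighting.
; Taking damage also sets PlayerFound and lowers CurrentHealth, which starts at MaxHealth.
; At zero health it sets IsDead and prints a death message, with no further death handling.
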(event `self.ReceiveBeginPlay`
  (set `self.CurrentHealth` (`self.MaxHealth`)))

(event `/Game/AI/AI/Blueprints/BP_DamageSystem.TakeDamage`
  (params (BoneName :type Name) (Damage :type "Float (single-precision)"))
  (set `self.PlayerFound` true)
  (bind _output_get (set `self.CurrentHealth` (- (`self.CurrentHealth`) Damage)))
  (if (<= _output_get 0.0)
    (set `self.isDead` true)
    (`KismetSystemLibrary.PrintString` "NPC has died!")))

(event `self.PawnSensing.OnSeePawn`
  (params (Pawn :type "Pawn Object Reference"))
  (cast `/Game/Character/Blueprints/BP_MainCharacter` Pawn)
  (`|ExecutionSequence`
    (:`then_0`
      (set `self.PlayerFound` true))
    (:`then_1`
      (`KismetSystemLibrary.RetriggerableDelay` 0.5)
      (set `self.PlayerFound` false))))

(fn `UserConstructionScript`)