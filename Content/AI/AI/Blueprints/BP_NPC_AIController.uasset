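; AI controller for BP_NPC that patrols between waypoints and chases the player to deal damage.
; Patrol alternates between the current waypoint and the next with timed pauses, never advancing the index here.
; A looping timer polls the pawn's PlayerFound flag to trigger the chase, and stops once the NPC is dead.
; The chase moves to the player, applies damage on arrival, then re-triggers itself after a short delay.
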(event `self.ReceiveBeginPlay`
  (bind _asbp_npc (cast `/Game/AI/AI/Blueprints/BP_NPC` (`self.K2_GetPawn`)))
  (set `self.AIReference` _asbp_npc)
  (set `self.WaypointsReference` (`/Game/AI/AI/Blueprints/BP_NPC.Waypoints` _asbp_npc))
  (bind _returnvalue (`KismetSystemLibrary.K2_SetTimer` null "CheckPlayer" 0.25 true))
  (set `self.Clear Time` _returnvalue)
  (`self.MoveToWaypoint`))

(event `OnChase`
  (bind _returnvalue (`GameplayStatics.GetPlayerCharacter` 0))
  (`|AIMoveTo` null (0.0 0.0 0.0) _returnvalue 50.0
    (:`OnSuccess`
      (`GameplayStatics.ApplyDamage` _returnvalue (`self.Base Damage`))
      (`KismetSystemLibrary.Delay` 0.5)
      (`self.OnChase`))))

(event `MoveToWaypoint`
  (`|AIMoveTo` null (0.0 0.0 0.0) (`|GetArrayItem` (`self.WaypointsReference`) (`self.CurrentWaypoint`)) 30.0
    (:`OnSuccess`
      (`KismetSystemLibrary.Delay` 5.0)
      (`|AIMoveTo` null (0.0 0.0 0.0) (`|GetArrayItem` (`self.WaypointsReference`) (+ (`self.CurrentWaypoint`) 1)) 30.0
        (:`then`
          (`KismetSystemLibrary.Delay` 5.0)
          (`self.MoveToWaypoint`))))))

(event `CheckPlayer`
  (bind _aireference (`self.AIReference`))
  (if (`/Game/AI/AI/Blueprints/BP_NPC.isDead` _aireference)
    (`KismetSystemLibrary.K2_ClearAndInvalidateTimerHandle` (`self.Clear Time`))
    (else
      (bind _output_get (set `self.PlayerFound` (`/Game/AI/AI/Blueprints/BP_NPC.PlayerFound` _aireference)))
      (if _output_get
        (`self.OnChase`)))))

(fn `UserConstructionScript`)