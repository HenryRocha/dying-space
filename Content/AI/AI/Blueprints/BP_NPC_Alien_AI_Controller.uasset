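; AI controller for the alien NPC that sends it to a waypoint and chases the player once found.
; On BeginPlay it caches the pawn and its waypoints, starts a looping timer, and issues a single move to the current waypoint, with nothing following the arrival delay.
; The timer polls the pawn's PlayerFound flag to re-issue a move toward the player, and clears itself when the alien is dead.
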(event `self.ReceiveBeginPlay`
  (bind _asbp_npc_alien (cast `/Game/AI/AI/Blueprints/BP_NPC_Alien` (`self.K2_GetPawn`)))
  (set `self.AIReference` _asbp_npc_alien)
  (set `self.Waypoints` (`/Game/AI/AI/Blueprints/BP_NPC_Alien.Waypoints` _asbp_npc_alien))
  (bind _returnvalue (`KismetSystemLibrary.K2_SetTimer` null "CheckPlayer" 0.25 true))
  (set `self.Clear Time` _returnvalue)
  (`|AIMoveTo` null (0.0 0.0 0.0) (`|GetArrayItem` (`self.Waypoints`) (`self.Current Waypoint`)) 30.0
    (:`OnSuccess`
      (`KismetSystemLibrary.Delay` 1.25))))

(event `OnChase`
  (`|AIMoveTo` null (0.0 0.0 0.0) (`GameplayStatics.GetPlayerCharacter` 0) 200.0))

(event `CheckPlayer`
  (bind _aireference (`self.AIReference`))
  (if (`/Game/AI/AI/Blueprints/BP_NPC_Alien.isDead` _aireference)
    (`KismetSystemLibrary.K2_ClearAndInvalidateTimerHandle` (`self.Clear Time`))
    (else
      (bind _output_get (set `self.PlayerFound` (`/Game/AI/AI/Blueprints/BP_NPC_Alien.PlayerFound` _aireference)))
      (if _output_get
        (`self.OnChase`)))))

(fn `UserConstructionScript`)