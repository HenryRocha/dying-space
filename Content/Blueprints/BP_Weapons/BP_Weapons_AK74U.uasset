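; AK-74U weapon Blueprint that handles firing and reloading for BP_MainCharacter.
; Fire prints and decrements the ammo count, switching the player character from firing to reloading when it runs out, and Reload refills it to the maximum.
; Each Fire call also runs a debug-drawn visibility trace from the player camera, even with no ammo, and the hit result is unused.
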(event `Event Fire`
  (`self.AmmoCounter`)
  (`self.ShootLineTrace`))

(event `Event Reload`
  (set `self.AmmoCount` (`self.MaxAmmo`)))

(fn `AmmoCounter`
  (`KismetSystemLibrary.PrintString` (`KismetStringLibrary.Conv_IntToString` (`self.AmmoCount`)))
  (if (> (`self.AmmoCount`) 0)
    (bind _result (`/Engine/EditorBlueprintResources/StandardMacros.DecrementInt` (`self.AmmoCount`))
      (:`  `
        (if (<= _result 0)
          (bind _asbp_main_character (cast `/Game/Character/Blueprints/BP_MainCharacter` (`GameplayStatics.GetPlayerCharacter` 0)))
          (set `/Game/Character/Blueprints/BP_MainCharacter.IsFiring` false _asbp_main_character)
          (set `/Game/Character/Blueprints/BP_MainCharacter.IsReloading` true _asbp_main_character))))))

(fn `ShootLineTrace`
  (bind _camera (`/Game/Character/Blueprints/BP_MainCharacter.Camera` (cast `/Game/Character/Blueprints/BP_MainCharacter` (`GameplayStatics.GetPlayerCharacter` 0) :!pure true)))
  (bind _returnvalue (`SceneComponent.K2_GetComponentLocation` _camera))
  (`KismetSystemLibrary.LineTraceSingle` :`Start` _returnvalue :`End` (+ _returnvalue (* (`SceneComponent.GetForwardVector` _camera) 25000.0)) :`TraceChannel` "TraceTypeQuery1" :`DrawDebugType` "ForDuration"))

(fn `UserConstructionScript`
  (`parent.UserConstructionScript`))