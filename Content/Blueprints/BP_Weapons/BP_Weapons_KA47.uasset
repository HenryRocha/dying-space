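; KA47 weapon Blueprint that handles firing, ammo and reloading for BP_MainCharacter.
; Fire decrements ammo, switching the character from firing to reloading at zero, then shoots without gating on ammo; Reload refills to MaxAmmo.
; Each shot traces from the player camera with debug drawing, plays a sound, and spawns an actor at the muzzle socket aimed at the impact point or trace end, aligning it with the crosshair line.
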(event `self.ReceiveBeginPlay`
  (`parent.ReceiveBeginPlay`)
  ;[1 1 1] Set initial ammo to be equal the max ammo, when the game starts
  (set `self.AmmoCount` (`self.Max Ammo`)))

(event `Event Fire`
  (`self.AmmoCounter`)
  (`self.ShootLineTrace`))

(event `Event Reload`
  (set `self.AmmoCount` (`self.Max Ammo`)))

(fn `AmmoCounter`
  (`KismetSystemLibrary.PrintString` (`KismetStringLibrary.Conv_IntToString` (`self.AmmoCount`)))
  (if (> (`self.AmmoCount`) 0)
    (bind _result (`/Engine/EditorBlueprintResources/StandardMacros.DecrementInt` (`self.AmmoCount`))
      (:`  `
        (if (<= _result 0)
          (bind _asbp_main_character (cast `/Game/Character/Blueprints/BP_MainCharacter` (`GameplayStatics.GetPlayerCharacter` 0)))
          (set `/Game/Character/Blueprints/BP_MainCharacter.IsFiring` false _asbp_main_character)
          (set `/Game/Character/Blueprints/BP_MainCharacter.IsReloading` true _asbp_main_character))))))

(fn `ShootLineTrace`
  (bind _returnvalue (`SceneComponent.GetSocketLocation` (`self.SkeletalMesh`) "MuzzleFlashSocket"))
  (bind _camera (`/Game/Character/Blueprints/BP_MainCharacter.Camera` (cast `/Game/Character/Blueprints/BP_MainCharacter` (`GameplayStatics.GetPlayerCharacter` 0) :!pure true)))
  (bind _returnvalue_2 (`SceneComponent.K2_GetComponentLocation` _camera))
  (bind (_outhit _returnvalue_3) (`KismetSystemLibrary.LineTraceSingle` :`Start` _returnvalue_2 :`End` (+ _returnvalue_2 (* (`SceneComponent.GetForwardVector` _camera) 25000.0)) :`TraceChannel` "TraceTypeQuery1" :`DrawDebugType` "ForDuration"))
  (`GameplayStatics.PlaySound2D` "/Game/Assets/Sounds/WeaponFire.WeaponFire" 1.0 1.0 0.0 null null)
  (bind (_bblockinghit _binitialoverlap _time _distance _location _impactpoint _normal _impactnormal _physmat _hitactor _hitcomponent _hitbonename _hititem _elementindex _faceindex _tracestart _traceend) (`GameplayStatics.BreakHitResult` _outhit))
  (set `self.Location` _location)
  (set `self.ImpactPoint` _impactpoint)
  (bind _output_get (set `self.ImpactNormal` _impactnormal))
  (bind _output_get_2 (set `self.HitActor` _hitactor))
  (set `self.HitComponent` _hitcomponent)
  (set `self.HitBoneName` _hitbonename)
  (set `self.TraceStart` _tracestart)
  (set `self.TraceEnd` _traceend)
  (set `self.HitNormalRotation` (`KismetMathLibrary.Conv_VectorToRotator` _output_get))
  (set `self.HitActorClass` (`GameplayStatics.GetObjectClass` _output_get_2))
  (`|SpawnActorFromClass` "/Game/Blueprints/BP_Weapons/BP_Projectiles.BP_Projectiles_C" (`KismetMathLibrary.MakeTransform` _returnvalue (`KismetMathLibrary.FindLookAtRotation` _returnvalue (`KismetMathLibrary.SelectVector` (`self.ImpactPoint`) (`self.TraceEnd`) _returnvalue_3))) "AlwaysSpawn" "OverrideRootScale" null null))

(fn `UserConstructionScript`
  (`parent.UserConstructionScript`))